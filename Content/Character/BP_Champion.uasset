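; BP_Champion is a champion character Blueprint with basic health, damage handling and a HUD health bar.
; On BeginPlay it creates the WP_HealthBar widget for the first player controller and adds it to the viewport.
; AnyDamage subtracts damage from Health, but the zero-health branch does nothing yet.
; A test key, M, damages the champion itself and plays a world camera shake at its location.
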(event EventBeginPlay
  ;[1 1 1] HealthBar Widget
  (bind _returnvalue (UserInterface|CreateWidget "/Game/Character/WP_HealthBar.WP_HealthBar_C" (Game|GetPlayerController 0)))
  (UserInterface|Viewport|AddtoViewport _returnvalue 0))

(event Collision|EventActorBeginOverlap
  (params (OtherActor :type Actor%20Object%20Reference)))

(event EventTick
  (params (DeltaSeconds :type Float%20%28single-precision%29)))

(event Game|Damage|EventAnyDamage
  (params (Damage :type Float%20%28single-precision%29) (DamageType :type Damage%20Type%20Object%20Reference) (InstigatedBy :type Controller%20Object%20Reference) (DamageCauser :type Actor%20Object%20Reference))
  ;[1 1 1] Damage Event TEST
  (Variables|Default|SetHealth (- (Variables|Default|GetHealth) Damage))
  (if (<= (Variables|Default|GetHealth) 0.0)
    _))

(event Input|KeyboardEvents|M
  (params (Key :type Key%20Structure :default "None"))
  ;[1 1 1] Damage Event TEST
  (:Pressed
    (Game|Damage|ApplyDamage self 1e+01 0 0)
    (Camera|PlayWorldCameraShake "/Game/Character/Camera/BP_CameraShake.BP_CameraShake_C" (Transformation|GetActorLocation) 0.0 5e+02)))

(event Input|KeyboardEvents|A
  (params (Key :type Key%20Structure :default "None")))

(fn ConstructionScript)